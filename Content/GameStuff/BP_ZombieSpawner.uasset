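; BP_ZombieSpawner is a spawner actor that continuously creates BP_ZombieCharacter enemies at its Sphere component's location and rotation.
; A timer started on BeginPlay calls SpawnZombie, which spawns a zombie, prints a debug message and re-arms the timer.
; The delay shrinks in steps as game time passes each minute mark up to three minutes, escalating pressure.
; Spawns are nudged clear of collisions, or skipped if still blocked.
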(event `self.ReceiveBeginPlay`
  (`KismetSystemLibrary.K2_SetTimerDelegate` (delegate `SpawnZombie`) 5.0))

(event `SpawnZombie`
  (bind _sphere (`self.Sphere`))
  (`|SpawnActorFromClass` "/Game/ZombieStuff/BP_ZombieCharacter.BP_ZombieCharacter_C" (`KismetMathLibrary.MakeTransform` (`SceneComponent.K2_GetComponentLocation` _sphere) (`SceneComponent.K2_GetComponentRotation` _sphere)) "AdjustIfPossibleButDontSpawnIfColliding" "MultiplyWithRoot" null null)
  (`KismetSystemLibrary.PrintString` "Spawn" true true (struct :`R` 1.0 :`B` 0.893243 :`A` 1.0))
  (bind _output_get (set `self.GottenGameTimeInSeconds` (`KismetSystemLibrary.GetGameTimeInSeconds`)))
  (if (< _output_get 60.0)
    (`KismetSystemLibrary.K2_SetTimerDelegate` (delegate `SpawnZombie`) 5.0)
    (elif (< (`self.GottenGameTimeInSeconds`) 120.0)
      (`KismetSystemLibrary.K2_SetTimerDelegate` (delegate `SpawnZombie`) 2.5)
      (elif (< (`self.GottenGameTimeInSeconds`) 180.0)
        (`KismetSystemLibrary.K2_SetTimerDelegate` (delegate `SpawnZombie`) 1.0)
        (else
          (`KismetSystemLibrary.K2_SetTimerDelegate` (delegate `SpawnZombie`) 0.5))))))

(fn `UserConstructionScript`)