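; BP_Turret is an auto-aiming turret that shoots BP_ZombieCharacter enemies while its energy lasts.
; A looping timer, or loss of target, picks a random zombie near the survivor, falling back to any zombie.
; Tick drains energy, turns the gun toward the target (spinning when none) and fires rate-limited bullets once roughly aligned.
; AddSupplies restores energy, shown on a camera-facing ammo bar widget.
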(event `UE5 Is Bugged :(`
  (`self.FindZombieTarget`))

(event `self.ReceiveBeginPlay`
  (`KismetSystemLibrary.K2_SetTimerDelegate` (delegate `UE5 Is Bugged :(`) 5.0 true 0.5)
  (set `self.Energy` (`self.MaxEnergy`))
  (bind _aswid_turret_ammo_bar (cast `/Game/GameStuff/Turret/WID_TurretAmmoBar` (`WidgetComponent.GetWidget` (`self.Widget`))))
  (bind _output_get (set `self.As WID Turret Ammo Bar` _aswid_turret_ammo_bar))
  (`/Game/GameStuff/Turret/WID_TurretAmmoBar.SetAmmo` _output_get (`self.Energy`) (`self.MaxEnergy`)))

(event `self.ReceiveTick`
  (params (DeltaSeconds :type "Float (single-precision)"))
  (`self.PointAmmoBarAtCamera`)
  (if (not (`self.OutOfEnergy`))
    (`self.UpdateRotation` DeltaSeconds)
    (`self.UpdateFire`)
    (set `self.Energy` (`KismetMathLibrary.FClamp` (- (`self.Energy`) (* (`self.EnergyDrain`) DeltaSeconds)) 0.0 (`self.MaxEnergy`)))
    (`/Game/GameStuff/Turret/WID_TurretAmmoBar.SetAmmo` (`self.As WID Turret Ammo Bar`) (`self.Energy`) (`self.MaxEnergy`))
    (set `self.OutOfEnergy` (<= (`self.Energy`) 0.0))))

(event `/Game/GameStuff/BI_Supplyable.AddSupplies`
  (params (SuppliesToAdd :type "Float (double-precision)"))
  (set `self.Energy` (`KismetMathLibrary.FClamp` (+ SuppliesToAdd (`self.Energy`)) 0.0 (`self.MaxEnergy`)))
  (set `self.OutOfEnergy` (<= (`self.Energy`) 0.0)))

(fn `FindZombieTarget`
  (returns (FoundZombie :type "/Game/ZombieStuff/BP_ZombieCharacter Object Reference"))
  (locals (NewLocalVar :type "Array of /Game/ZombieStuff/BP_ZombieCharacter Object Reference"))
  (bind _newlocalvar (`local.NewLocalVar`))
  (bind _newlocalvar_2 (`local.NewLocalVar`))
  (if (not (`self.OutOfEnergy`))
    ;[1 1 1] Get list of zombies close to the survivor
    (bind _outactors (`GameplayStatics.GetAllActorsOfClass` "/Game/ZombieStuff/BP_ZombieCharacter.BP_ZombieCharacter_C"))
    (for _array_element _outactors
      (bind _distancetosurvivor (`/Game/ZombieStuff/BP_ZombieCharacter.GetDistanceToSurvivor` _array_element))
      (if (<= _distancetosurvivor 250.0)
        (`KismetArrayLibrary.Array_Add` _newlocalvar_2 _array_element)))
    (if (> (`KismetArrayLibrary.Array_Length` _newlocalvar_2) 0)
      (set `self.TargetZombie` (`|GetArrayItem` _newlocalvar (`KismetMathLibrary.RandomIntegerInRange` 0 (- (`KismetArrayLibrary.Array_Length` _newlocalvar) 1))))
      (else
        ;[1 1 1] FindRandomTarget
        (bind _outactors_2 (`GameplayStatics.GetAllActorsOfClass` "/Game/ZombieStuff/BP_ZombieCharacter.BP_ZombieCharacter_C"))
        (bind _output_get (set `self.TargetZombie` (`|GetArrayItem` _outactors_2 (`KismetMathLibrary.RandomIntegerInRange` 0 (- (`KismetArrayLibrary.Array_Length` _outactors_2) 1)))))))
    (return _output_get)))

(fn `FireBullet`
  (bind (_returnvalue_location _returnvalue_rotation) (`KismetMathLibrary.BreakTransform` (`SceneComponent.K2_GetComponentToWorld` (`self.GunBase`))))
  (if (`KismetSystemLibrary.IsValid` (`self.TargetZombie`))
    (set `self.TimeOfLastFire` (`KismetSystemLibrary.GetGameTimeInSeconds`))
    (bind _returnvalue (`|SpawnActorFromClass` "/Game/GameStuff/Turret/BP_TurretBullet.BP_TurretBullet_C" (`KismetMathLibrary.MakeTransform` _returnvalue_location _returnvalue_rotation) "Undefined" "MultiplyWithRoot" null null))
    (if (`KismetSystemLibrary.IsValid` _returnvalue)
      (`/Game/GameStuff/Turret/BP_TurretBullet.SetBulletDamage` _returnvalue (`self.DamageAmount`)))))

(fn `PointAmmoBarAtCamera`
  (bind _widget (`self.Widget`))
  (`SceneComponent.K2_SetWorldRotation` _widget (`KismetMathLibrary.FindLookAtRotation` (`SceneComponent.K2_GetComponentLocation` _widget) (`SceneComponent.K2_GetComponentLocation` (`PlayerCameraManager.TransformComponent` (`GameplayStatics.GetPlayerCameraManager` 0)))) false false))

(fn `UpdateFire`
  (if (>= (- (`KismetSystemLibrary.GetGameTimeInSeconds`) (`self.TimeOfLastFire`)) (`self.RateOfFire`))
    (if (`KismetSystemLibrary.IsValid` (`self.TargetZombie`))
      (if (> (`KismetMathLibrary.Dot_VectorVector` (`KismetMathLibrary.GetDirectionUnitVector` (`SceneComponent.K2_GetComponentLocation` (`self.GunBase`)) (`self.K2_GetActorLocation` (`self.TargetZombie`))) (`SceneComponent.GetForwardVector` (`self.GunBase`))) 0.9)
        (`self.FireBullet`))
      (else
        (`self.FindZombieTarget`)))))

(fn `UpdateRotation`
  (params (`Delta Time` :type "Float (double-precision)"))
  (bind (_returnvalue_roll _returnvalue_pitch _returnvalue_yaw) (`KismetMathLibrary.BreakRotator` (`SceneComponent.K2_GetComponentRotation` (`self.GunBase`))))
  (bind (_returnvalue_x _returnvalue_y _returnvalue_z) (`KismetMathLibrary.BreakVector` (`SceneComponent.K2_GetComponentLocation` (`Character.Mesh` (`self.TargetZombie`)))))
  (if (`KismetSystemLibrary.IsValid` (`self.TargetZombie`))
    (`SceneComponent.K2_SetWorldRotation` (`self.GunBase`) (`KismetMathLibrary.RInterpTo_Constant` (`SceneComponent.K2_GetComponentRotation` (`self.GunBase`)) (`KismetMathLibrary.FindLookAtRotation` (`SceneComponent.K2_GetComponentLocation` (`self.GunBase`)) (`KismetMathLibrary.MakeVector` _returnvalue_x _returnvalue_y (+ _returnvalue_z 100.0))) `Delta Time` (`self.Interp Speed`)) false false)
    (return)
    (else
      ;[1 1 1] If no valid zombie target, just spin
      (`SceneComponent.K2_SetWorldRotation` (`self.GunBase`) (`KismetMathLibrary.RInterpTo_Constant` (`KismetMathLibrary.MakeRotator` _returnvalue_roll _returnvalue_pitch _returnvalue_yaw) (`KismetMathLibrary.MakeRotator` _returnvalue_roll _returnvalue_pitch (+ _returnvalue_yaw 10.0)) `Delta Time` (`self.Interp Speed`)) false false)
      (return))))

(fn `UserConstructionScript`)