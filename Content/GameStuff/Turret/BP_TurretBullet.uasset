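; Turret bullet projectile that damages zombies on sphere overlap, with damage set through a SetBulletDamage event.
; Overlaps are filtered by interface: turret and zombie-damageable actors are ignored, and any other non-zombie actor destroys the bullet.
; Zombie hits send a bullet damage message, spawn a Niagara hit effect facing opposite the bullet's rotation, then destroy it.
; The Fly function is empty.
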(event `self.ReceiveBeginPlay`)

(event `self.Sphere.OnComponentBeginOverlap`
  (params (OverlappedComponent :type "PrimitiveComponent Object Reference") (OtherActor :type "Actor Object Reference") (OtherComp :type "PrimitiveComponent Object Reference") (OtherBodyIndex :type Integer) (bFromSweep :type Boolean) (SweepResult :type "HitResult Structure (by ref)"))
  (bind (_returnvalue_location _returnvalue_rotation _returnvalue_scale) (`KismetMathLibrary.BreakTransform` (`SceneComponent.K2_GetComponentToWorld` (`self.Sphere`))))
  (if (not (`KismetSystemLibrary.DoesImplementInterface` OtherActor "/Game/GameStuff/Turret/BI_TurretInterface.BI_TurretInterface_C"))
    (if (`KismetSystemLibrary.DoesImplementInterface` OtherActor "/Game/ZombieStuff/BI_ZombieInterface.BI_ZombieInterface_C")
      (message `/Game/ZombieStuff/BI_ZombieInterface.TakeBulletDamage` OtherActor (`self.Damage`))
      (`NiagaraFunctionLibrary.SpawnSystemAtLocation` "/Game/GameStuff/Turret/NS_ZombieHitParticle.NS_ZombieHitParticle" _returnvalue_location (`KismetMathLibrary.NegateRotator` _returnvalue_rotation) _returnvalue_scale)
      (`self.K2_DestroyActor`)
      (elif (not (`KismetSystemLibrary.DoesImplementInterface` OtherActor "/Game/ZombieStuff/BI_TakeZombieDamage.BI_TakeZombieDamage_C"))
        (`self.K2_DestroyActor`)))))

(event `SetBulletDamage`
  (params (Damage :type "Float (double-precision)"))
  (set `self.Damage` Damage))

(fn `Fly`
  (params (ForwardVector :type "Vector Structure")))

(fn `UserConstructionScript`)