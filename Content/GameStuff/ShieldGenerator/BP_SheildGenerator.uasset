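; Shield generator actor whose energy drains constantly, is refilled by supplies and is reduced by damage, including zombie attacks.
; The shield drops at zero energy and restarts above it, toggling the sphere visual and its response on a custom collision channel between Block and Overlap.
; Overlap events track zombies via interface, and restarting deals massive bullet damage to those inside.
; A widget bar shows energy and faces the camera each tick.
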(event `self.ReceiveBeginPlay`
  (bind _aswid_sheild_energy_bar (cast `/Game/GameStuff/ShieldGenerator/WID_SheildEnergyBar` (`WidgetComponent.GetWidget` (`self.Widget`))))
  (set `self.As WID Sheild Energy Bar` _aswid_sheild_energy_bar))

(event `self.ReceiveTick`
  (params (DeltaSeconds :type "Float (single-precision)"))
  (bind _maxenergy (`self.MaxEnergy`))
  (bind _output_get (set `self.Energy` (`KismetMathLibrary.FClamp` (- (`self.Energy`) (* DeltaSeconds 20.0)) 0.0 _maxenergy)))
  (`/Game/GameStuff/ShieldGenerator/WID_SheildEnergyBar.SetEnergy` (`self.As WID Sheild Energy Bar`) _output_get _maxenergy)
  (`self.PointEnergyBarAtCamera`)
  (if (<= (`self.Energy`) 0.0) :!label _label
    (if (`self.IsSheildUp`)
      (`self.ShutDownSheild`))
    (elif (not (`self.IsSheildUp`))
      (`self.StartUpSheild`))))

(event `/Game/GameStuff/ShieldGenerator/BI_SheildInterface.ApplyDamage`
  (params (Damage :type "Float (double-precision)") (AttackingActor :type "Actor Object Reference"))
  (set `self.Energy` (- (`self.Energy`) Damage))
  (goto _label))

(event `/Game/GameStuff/ShieldGenerator/BI_SheildInterface.AddEnergy`
  (params (SuppliesIn :type "Float (double-precision)")))

(event `/Game/GameStuff/BI_Supplyable.AddSupplies`
  (params (SuppliesToAdd :type "Float (double-precision)"))
  (set `self.Energy` (`KismetMathLibrary.FClamp` (+ (* SuppliesToAdd 20.0) (`self.Energy`)) 0.0 (`self.MaxEnergy`))))

(event `/Game/ZombieStuff/BI_TakeZombieDamage.TakeZombieDamage`
  (params (DamageAmount :type "Float (double-precision)"))
  (set `self.Energy` (`KismetMathLibrary.FClamp` (- (`self.Energy`) DamageAmount) 0.0 (`self.MaxEnergy`)))
  (if (<= (`self.Energy`) 0.0)
    (if (`self.IsSheildUp`)
      (`self.ShutDownSheild`))
    (elif (not (`self.IsSheildUp`))
      (`self.StartUpSheild`))))

(event `self.Sphere.OnComponentBeginOverlap`
  (params (OverlappedComponent :type "PrimitiveComponent Object Reference") (OtherActor :type "Actor Object Reference") (OtherComp :type "PrimitiveComponent Object Reference") (OtherBodyIndex :type Integer) (bFromSweep :type Boolean) (SweepResult :type "HitResult Structure (by ref)"))
  (if (`KismetSystemLibrary.DoesImplementInterface` OtherActor "/Game/ZombieStuff/BI_ZombieInterface.BI_ZombieInterface_C")
    (`KismetArrayLibrary.Array_Add` (`self.Other Actor`) OtherActor)))

(event `self.Sphere.OnComponentEndOverlap`
  (params (OverlappedComponent :type "PrimitiveComponent Object Reference") (OtherActor :type "Actor Object Reference") (OtherComp :type "PrimitiveComponent Object Reference") (OtherBodyIndex :type Integer))
  (if (`KismetSystemLibrary.DoesImplementInterface` OtherActor "/Game/ZombieStuff/BI_ZombieInterface.BI_ZombieInterface_C")
    (`KismetArrayLibrary.Array_RemoveItem` (`self.Other Actor`) OtherActor)))

(fn `PointEnergyBarAtCamera`
  (bind _widget (`self.Widget`))
  (`SceneComponent.K2_SetWorldRotation` _widget (`KismetMathLibrary.FindLookAtRotation` (`SceneComponent.K2_GetComponentLocation` _widget) (`SceneComponent.K2_GetComponentLocation` (`PlayerCameraManager.TransformComponent` (`GameplayStatics.GetPlayerCameraManager` 0)))) false false))

(fn `ShutDownSheild`
  (bind _sphere (`self.Sphere`))
  (`SceneComponent.SetVisibility` (`self.ShieldSphere`) false false)
  (`SceneComponent.SetVisibility` _sphere false false)
  (`PrimitiveComponent.SetCollisionResponseToChannel` _sphere "ECC_GameTraceChannel1" "ECR_Overlap")
  (set `self.IsSheildUp` false))

(fn `StartUpSheild`
  (for _array_element (`self.Other Actor`)
    (message `/Game/ZombieStuff/BI_ZombieInterface.TakeBulletDamage` _array_element 100000.0))
  (`SceneComponent.SetVisibility` (`self.ShieldSphere`) true false)
  (`PrimitiveComponent.SetCollisionResponseToChannel` (`self.Sphere`) "ECC_GameTraceChannel1" "ECR_Block")
  (set `self.IsSheildUp` true)
  (return))

(fn `UserConstructionScript`)