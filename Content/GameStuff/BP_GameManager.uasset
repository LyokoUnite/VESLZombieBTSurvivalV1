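; Game manager that runs the match clock and awards time-based score to the local player.
; On BeginPlay it caches the player as either the third-person character or, failing that cast, a spectator pawn, then starts a one-second looping timer.
; Each tick advances seconds and minutes, adds a per-second or per-minute score, and pushes time and score to that pawn's UI through parallel character and spectator functions.
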(event `self.ReceiveBeginPlay`
  (bind _asbp_third_person_character (cast `/Game/ThirdPerson/Blueprints/BP_ThirdPersonCharacter` (`GameplayStatics.GetPlayerCharacter` 0))
    (:`then`
      (bind _output_get (set `self.As BP Third Person Character` _asbp_third_person_character))
      (`/Engine/EditorBlueprintResources/StandardMacros.IsValid` _output_get
        (:`Is Valid`
          (`KismetSystemLibrary.K2_SetTimerDelegate` (delegate `Clock`) 1.0 true 1.0))))
    (:`CastFailed`
      (bind _asbp_spectator_pawn (cast `/Game/ThirdPerson/Blueprints/BP_SpectatorPawn` (`GameplayStatics.GetPlayerPawn` 0)))
      (set `self.As BP Spectator Pawn` _asbp_spectator_pawn)
      (`KismetSystemLibrary.K2_SetTimerDelegate` (delegate `SpectatorClock`) 1.0 true 1.0))))

(event `Clock`
  (if (>= (`self.TimeInSeconds`) 59)
    (set `self.TimeInSeconds` 0)
    (`/Engine/EditorBlueprintResources/StandardMacros.IncrementInt` (`self.TimeInMinutes`)
      (:`  `
        (`self.UpdateScorerUI` (`self.ScoreForMinute`))))
    (else
      (`/Engine/EditorBlueprintResources/StandardMacros.IncrementInt` (`self.TimeInSeconds`)
        (:`  `
          (`self.UpdateScorerUI` (`self.ScoreForSecond`))))))
  (`self.UpdateTimerUI`))

(event `SpectatorClock`
  (if (>= (`self.TimeInSeconds`) 59)
    (set `self.TimeInSeconds` 0)
    (`/Engine/EditorBlueprintResources/StandardMacros.IncrementInt` (`self.TimeInMinutes`)
      (:`  `
        (`self.UpdateScorerUI_Spectator` (`self.ScoreForMinute`))))
    (else
      (`/Engine/EditorBlueprintResources/StandardMacros.IncrementInt` (`self.TimeInSeconds`)
        (:`  `
          (`self.UpdateScorerUI_Spectator` (`self.ScoreForSecond`))))))
  (`self.UpdateTimerUI_Spectator`))

(fn `UpdateScorerUI`
  (params (ScoreToAdd :type Integer))
  (`/Game/ThirdPerson/Blueprints/BP_ThirdPersonCharacter.UpdateScoreUI` (`self.As BP Third Person Character`) ScoreToAdd)
  (return))

(fn `UpdateScorerUI_Spectator`
  (params (ScoreToAdd :type Integer))
  (`/Game/ThirdPerson/Blueprints/BP_SpectatorPawn.UpdateScoreUI` (`self.As BP Spectator Pawn`) ScoreToAdd)
  (return))

(fn `UpdateTimerUI`
  (`/Game/ThirdPerson/Blueprints/BP_ThirdPersonCharacter.UpdateTimeUI` (`self.As BP Third Person Character`) (`self.TimeInMinutes`) (`self.TimeInSeconds`))
  (return))

(fn `UpdateTimerUI_Spectator`
  (`/Game/ThirdPerson/Blueprints/BP_SpectatorPawn.UpdateTimeUI` (`self.As BP Spectator Pawn`) (`self.TimeInMinutes`) (`self.TimeInSeconds`))
  (return))

(fn `UserConstructionScript`)