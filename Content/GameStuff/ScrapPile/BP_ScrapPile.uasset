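; BP_ScrapPile is a scrap pickup that hands out supplies in chunks from a limited pool and refills after running dry.
; CollectSupplies returns up to a fixed amount, and UpdateScale hides the whole pile at zero rather than shrinking it, as scaling is disconnected.
; While empty, Tick runs a timer that restores the full pool and visibility.
; A sphere overlap counts nearby actors implementing BI_ZombieInterface.
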(event `self.ReceiveBeginPlay`
  (set `self.StartingScale` (`SceneComponent.K2_GetComponentScale` (`self.Cube`))))

(event `self.ReceiveTick`
  (params (DeltaSeconds :type "Float (single-precision)"))
  (if (not (`self.HasScrap`))
    (bind _output_get (set `self.ResupplyMeter` (+ DeltaSeconds (`self.ResupplyMeter`))))
    (if (>= _output_get 7.0)
      (`self.ResupplyScrap`))))

(event `self.Sphere.OnComponentBeginOverlap`
  (params (OverlappedComponent :type "PrimitiveComponent Object Reference") (OtherActor :type "Actor Object Reference") (OtherComp :type "PrimitiveComponent Object Reference") (OtherBodyIndex :type Integer) (bFromSweep :type Boolean) (SweepResult :type "HitResult Structure (by ref)"))
  (if (`KismetSystemLibrary.DoesImplementInterface` OtherActor "/Game/ZombieStuff/BI_ZombieInterface.BI_ZombieInterface_C")
    (bind _result (`/Engine/EditorBlueprintResources/StandardMacros.IncrementInt` (`self.SurroundingZombies`)))))

(event `self.Sphere.OnComponentEndOverlap`
  (params (OverlappedComponent :type "PrimitiveComponent Object Reference") (OtherActor :type "Actor Object Reference") (OtherComp :type "PrimitiveComponent Object Reference") (OtherBodyIndex :type Integer))
  (if (`KismetSystemLibrary.DoesImplementInterface` OtherActor "/Game/ZombieStuff/BI_ZombieInterface.BI_ZombieInterface_C")
    (bind _result (`/Engine/EditorBlueprintResources/StandardMacros.DecrementInt` (`self.SurroundingZombies`)))))

(fn `CollectSupplies`
  (returns (AmountGiven :type "Float (double-precision)"))
  (if (<= (`self.SupplyPool`) 20.0)
    (bind _output_get (set `self.AmountToGive` (`self.SupplyPool`)))
    (set `self.SupplyPool` 0.0)
    (set `self.HasScrap` false)
    (`self.UpdateScale`)
    (return _output_get)
    (else
      (set `self.AmountToGive` 20.0)
      (set `self.SupplyPool` (`KismetMathLibrary.FClamp` (- (`self.SupplyPool`) (`self.AmountToGive`)) 0.0 100.0))
      (set `self.HasScrap` true)
      (`self.UpdateScale`)
      (return 20.0))))

(fn `ResupplyScrap`
  (set `self.SupplyPool` (`self.SupplyPoolMax`))
  (set `self.HasScrap` true)
  (set `self.ResupplyMeter` 0.0)
  (`self.UpdateScale`))

(fn `UpdateScale`
  (if (<= (`self.SupplyPool`) 0.0)
    (`SceneComponent.SetHiddenInGame` (`self.DefaultSceneRoot`) true true)
    (else
      (`SceneComponent.SetHiddenInGame` (`self.DefaultSceneRoot`) false true))))

(fn `UserConstructionScript`)