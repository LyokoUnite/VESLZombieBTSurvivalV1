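; AI controller for survivor characters that runs the survivor behavior tree on possess and supplies its blackboard.
; On BeginPlay it finds the shield generator actor and writes it, along with a hardcoded world position, to the blackboard.
; Update events copy health, supplies and nearby zombie count into blackboard keys, and spread an array of scrap objects across numbered ScrapPile keys.
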(event `self.ReceivePossess`
  (params (PossessedPawn :type "Pawn Object Reference"))
  (`self.RunBehaviorTree` "/Game/SurvivorStuff/BT_SurvivorBehaviorTree.BT_SurvivorBehaviorTree"))

(event `self.ReceiveBeginPlay`
  (bind _returnvalue (`GameplayStatics.GetActorOfClass` "/Game/GameStuff/ShieldGenerator/BP_SheildGenerator.BP_SheildGenerator_C"))
  (bind _output_get (set `self.ShieldActor` _returnvalue))
  (`BlackboardComponent.SetValueAsObject` (`AIBlueprintHelperLibrary.GetBlackboard` null) (`self.Shield Key Name`) _output_get)
  (`BlackboardComponent.SetValueAsVector` (`AIBlueprintHelperLibrary.GetBlackboard` null) (`KismetStringLibrary.Conv_StringToName` "VectorKey") (`KismetMathLibrary.MakeVector` 2360.0 5520.0 50.0)))

(event `UpdateSurvivorBTHealth`
  (params (Health :type "Float (double-precision)"))
  (`BlackboardComponent.SetValueAsFloat` (`self.Blackboard`) (`self.Health Key Name`) Health))

(event `UpdateSurvivorBTSupplies`
  (params (Supplies :type "Float (double-precision)"))
  (`BlackboardComponent.SetValueAsFloat` (`self.Blackboard`) (`self.Supplies Key Name`) Supplies))

(event `UpdateSurvivorBTCloseZombies`
  (params (NumberOfCloseZombies :type Integer))
  (`BlackboardComponent.SetValueAsInt` (`self.Blackboard`) (`self.Close Zombies Key Name`) NumberOfCloseZombies))

(event `UpdateSurvivorBTScrapObjects`
  (params (NewParam :type "Array of Actor Object Reference"))
  (for (_array_element _array_index) NewParam
    (`BlackboardComponent.SetValueAsObject` (`self.Blackboard`) (`KismetStringLibrary.Conv_StringToName` (`KismetStringLibrary.Concat_StrStr` "ScrapPile" (`KismetStringLibrary.Conv_IntToString` (+ _array_index 1)))) _array_element)))

(fn `UserConstructionScript`)