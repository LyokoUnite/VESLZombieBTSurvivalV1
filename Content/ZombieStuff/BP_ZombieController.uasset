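; AI controller for zombies that runs BT_ZombieTree on possession and feeds its Blackboard.
; AI perception sets line of sight and target for actors tagged Survivor; other updates start a timer that clears both unless a sighting cancels it.
; Each tick, distance checks against the cached player character and shield generator set the attack flags.
; Shield attacks require the shield up and the zombie within a minimum-to-maximum distance band.
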(event `self.ReceiveBeginPlay`
  (bind _returnvalue (`GameplayStatics.GetActorOfClass` "/Game/ThirdPerson/Blueprints/BP_ThirdPersonCharacter.BP_ThirdPersonCharacter_C"))
  (set `self.Survivor` _returnvalue)
  (bind _returnvalue_2 (`GameplayStatics.GetActorOfClass` "/Game/GameStuff/ShieldGenerator/BP_SheildGenerator.BP_SheildGenerator_C"))
  (set `self.Shield` _returnvalue_2))

(event `self.ReceiveTick`
  (params (DeltaSeconds :type "Float (single-precision)"))
  (`self.CheckIfInRange`))

(event `self.ReceivePossess`
  (params (PossessedPawn :type "Pawn Object Reference"))
  (`self.RunBehaviorTree` "/Game/ZombieStuff/BT_ZombieTree.BT_ZombieTree"))

(event `self.AIPerception.OnTargetPerceptionUpdated`
  (params (Actor :type "Actor Object Reference") (Stimulus :type "AIStimulus Structure"))
  (bind _blackboard (`self.Blackboard`))
  (if (and (`self.ActorHasTag` Actor "Survivor") (`.bSuccessfullySensed` (break `AIStimulus` Stimulus)))
    (`KismetSystemLibrary.K2_ClearAndInvalidateTimerHandle` (`self.EnemyTimer`))
    (`BlackboardComponent.SetValueAsBool` _blackboard (`self.HasLineOfSight`) true)
    (`BlackboardComponent.SetValueAsObject` _blackboard (`self.SurvivorActor`) Actor)
    (else
      (bind _returnvalue (`KismetSystemLibrary.K2_SetTimerDelegate` (delegate `StartEnemyTimer`) (`self.LineOfSightTimer`)))
      (set `self.EnemyTimer` _returnvalue))))

(event `StartEnemyTimer`
  (bind _blackboard (`self.Blackboard`))
  (`BlackboardComponent.SetValueAsBool` _blackboard (`self.HasLineOfSight`) false)
  (`BlackboardComponent.SetValueAsObject` _blackboard (`self.SurvivorActor`) null))

(fn `CheckIfInRange`
  (bind _returnvalue (`self.GetDistanceTo` (`self.Shield`) (`self.K2_GetPawn`)))
  (`|ExecutionSequence`
    (:`then_0`
      (`BlackboardComponent.SetValueAsBool` (`AIBlueprintHelperLibrary.GetBlackboard` null) (`self.CanAttackShield`) (and (and (<= _returnvalue (`self.AttackDistanceFromShield`)) (>= _returnvalue 700.0)) (`/Game/GameStuff/ShieldGenerator/BP_SheildGenerator.IsSheildUp` (`self.Shield`)))))
    (:`then_1`
      (`BlackboardComponent.SetValueAsBool` (`AIBlueprintHelperLibrary.GetBlackboard` null) (`self.CanAttackSurvivor`) (<= (`self.GetDistanceTo` (`self.Survivor`) (`self.K2_GetPawn`)) 150.0)))))

(fn `UserConstructionScript`)